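; Game instance for the fighter game that switches between the main menu and gameplay through a state machine.
; On Init it sets up the machine, binds its state-change event and enters MainMenu.
; Main Menu opens the menu map, unpauses and shows a reusable InitialSplash widget with UI-only input and cursor.
; In Game clears widgets and loads the side-scroller map; both states set input mode after a short post-load delay.
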(event `self.ReceiveInit`
  (bind _statemachine (`self.StateMachine`))
  (set `BasicStateMachine.States` (`self.InitialState`) _statemachine)
  (add `BasicStateMachine.OnStateChanged` _statemachine (delegate `CustomEvent_0`))
  (`BasicStateMachine.SetState` _statemachine "MainMenu"))

(event `CustomEvent_0`
  (params (NewState :type String) (OldState :type String))
  (bind _returnvalue (`GameplayStatics.GetPlayerController` 0))
  (bind _returnvalue_2 (`GameplayStatics.GetPlayerController` 0))
  (bind _mainmenuscreen (`self.MainMenuScreen`))
  (switch `string` NewState
    (:`MainMenu`
      ;[1 1 1] Main Menu
      (`GameplayStatics.OpenLevel` "MainMenuMap")
      (`KismetSystemLibrary.Delay` 0.2)
      (`GameplayStatics.SetGamePaused` false)
      (if (not (`KismetSystemLibrary.IsValid` (`self.MainMenuScreen`)))
        (bind _returnvalue_3 (`|CreateWidget` "/Game/Widgets/MainMenu/InitialSplash.InitialSplash_C"))
        (set `self.MainMenuScreen` _returnvalue_3))
      (`UserWidget.AddToViewport` _mainmenuscreen 0)
      (`WidgetBlueprintLibrary.SetInputMode_UIOnlyEx` _returnvalue_2 _mainmenuscreen)
      (set `PlayerController.bShowMouseCursor` true _returnvalue_2))
    (:`InGame`
      ;[1 1 1] In Game
      (`WidgetLayoutLibrary.RemoveAllWidgets`)
      (`GameplayStatics.OpenLevel` "SideScrollerExampleMap")
      (`KismetSystemLibrary.Delay` 0.2)
      (`WidgetBlueprintLibrary.SetInputMode_GameOnly` _returnvalue)
      (set `PlayerController.bShowMouseCursor` false _returnvalue))))